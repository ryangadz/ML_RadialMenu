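; BP_MenuIcon is a menu icon actor that shows a configurable mesh and animates when selected.
; The construction script assigns the mesh and creates a dynamic M_BasicMagicLight material with full desaturation and a configurable hue shift.
; ScaleUp sets Selected and plays a timeline driving scale and desaturation, while ScaleDown clears it and reverses the timeline.
; Tick spins the mesh around yaw while selected; the HueShift event is empty.
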(event `self.ReceiveBeginPlay`
  (set `self.InitialTime` (`KismetSystemLibrary.GetGameTimeInSeconds`)))

(event `HueShift`
  (params (Shift :type "Float (double-precision)")))

(event `self.ReceiveTick`
  (params (DeltaSeconds :type "Float (single-precision)"))
  (if (`self.Selected?`)
    (`SceneComponent.K2_AddRelativeRotation` (`self.IconMeshComponent`) (`KismetMathLibrary.MakeRotator` 0.0 0.0 (* DeltaSeconds 360.0)) false false)))

(event `ScaleUp`
  (set `self.Selected?` true)
  (bind (_direction _scale _desaturation) (`Timeline|Timeline_0` :!via `PlayFromStart` :!label _label)
    (:`Update`
      (`SceneComponent.SetRelativeScale3D` (`self.IconMeshComponent`) (`KismetMathLibrary.Conv_DoubleToVector` _scale))
      (`MaterialInstanceDynamic.SetScalarParameterValue` (`self.DynamicMaterial`) "Desaturation" _desaturation))))

(event `ScaleDown`
  (set `self.Selected?` false)
  (goto _label :!via `Reverse`))

(fn `UserConstructionScript`
  (bind _iconmeshcomponent (`self.IconMeshComponent`))
  (`StaticMeshComponent.SetStaticMesh` _iconmeshcomponent (`self.StaticMesh`))
  (bind _returnvalue (`PrimitiveComponent.CreateDynamicMaterialInstance` _iconmeshcomponent 0 "/Game/MaterialLibrary/Paint/M_BasicMagicLight.M_BasicMagicLight" "None"))
  (bind _output_get (set `self.DynamicMaterial` _returnvalue))
  (`MaterialInstanceDynamic.SetScalarParameterValue` _output_get "Desaturation" 1.0)
  (`MaterialInstanceDynamic.SetScalarParameterValue` (`self.DynamicMaterial`) "HueShift" (`self.ColorHueShift`))
  (`MaterialInstanceDynamic.SetScalarParameterValue` _output_get "HueShift" (`self.ColorHueShift`)))