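; BP_RadialMenu is a radial selection menu actor that shows one 3D icon per SubPawn class and highlights the choice under a thumb position.
; BuildRadialIcons spawns BP_MenuIcon actors evenly around a circle, with mesh from each class's Type default and hue from angle.
; A dynamic material receives thumb location and selection state, while hover events scale icons up or down.
; Reveal and Hide scale the whole actor through a timeline.
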(event `self.ReceiveBeginPlay`)

(event `self.ReceiveTick`
  (params (DeltaSeconds :type "Float (single-precision)")))

(event `UpdateMaterial`
  (params (ThumbLocation :type "Vector2D Structure") (NullSelect :type Boolean) (HoverIndex :type Integer))
  (bind _returnvalue (`KismetMathLibrary.Conv_BoolToDouble` NullSelect))
  (bind _menugraphicmaterial (`self.MenuGraphicMaterial`))
  (`MaterialInstanceDynamic.SetVectorParameterValue` (`self.MenuGraphicMaterial`) "ThumbLocation" (make `LinearColor` ThumbLocation_X (* ThumbLocation_Y -1.0) 0.0 1.0))
  (if NullSelect
    (`MaterialInstanceDynamic.SetScalarParameterValue` _menugraphicmaterial "NullSelect" _returnvalue)
    (else
      (`MaterialInstanceDynamic.SetScalarParameterValue` _menugraphicmaterial "NullSelect" _returnvalue)
      (`MaterialInstanceDynamic.SetScalarParameterValue` _menugraphicmaterial "Selected" (`KismetMathLibrary.Conv_IntToDouble` HoverIndex)))))

(event `CustomEvent_0`)

(event `Deselect`
  (bind _output (`|GetArrayItem` (`self.IconArray`) (`self.HoverIconCurrent`)))
  (`/Engine/EditorBlueprintResources/StandardMacros.IsValid` _output
    (:`Is Valid`
      (`/Game/Core/Interactables/BP_MenuIcon.ScaleDown` _output))
    (:`Is Not Valid`
      _))
  (set `self.HoverIconCurrent` -1))

(event `ResizeIcons`
  (params (HoverIdex :type Integer))
  (bind _output (`|GetArrayItem` (`self.IconArray`) (`self.HoverIconCurrent`)))
  (bind _output_2 (`|GetArrayItem` (`self.IconArray`) HoverIdex))
  (if (!= HoverIdex (`self.HoverIconCurrent`))
    (`/Engine/EditorBlueprintResources/StandardMacros.IsValid` _output_2
      (:`Is Valid`
        (`/Game/Core/Interactables/BP_MenuIcon.ScaleUp` _output_2))
      (:`Is Not Valid`
        _))
    (`/Engine/EditorBlueprintResources/StandardMacros.IsValid` _output
      (:`Is Valid`
        (`/Game/Core/Interactables/BP_MenuIcon.ScaleDown` _output))
      (:`Is Not Valid`
        _))
    (set `self.HoverIconCurrent` HoverIdex)))

(event `Reveal`
  (bind (_direction _newtrack_0) (`Timeline|ScaleActor` :!via `PlayFromStart` :!label _label)
    (:`Update`
      (`self.SetActorRelativeScale3D` self (`KismetMathLibrary.Conv_DoubleToVector` _newtrack_0)))))

(event `Hide`
  (goto _label :!via `Reverse`))

(fn `AddNewIcon`
  (params (IconIndex :type Integer) (SubPawns :type "Array of /Game/Core/Characters/BP_MasterPawn Class Reference"))
  (bind _toolradius (`self.ToolRadius`))
  (bind _returnvalue (* (`local.IconIndex`) (`self.AngleBetweenIcons`)))
  (bind _returnvalue_2 (`AddComponent|NODE_AddSceneComponent-0` :`RelativeTransform` (`KismetMathLibrary.MakeTransform` (`KismetMathLibrary.MakeVector` (+ (* (`KismetMathLibrary.DegCos` _returnvalue) _toolradius) -2.0) (* (`KismetMathLibrary.DegSin` _returnvalue) _toolradius)))))
  (bind _returnvalue_3 (`|SpawnActorFromClass` "/Game/Core/Interactables/BP_MenuIcon.BP_MenuIcon_C" (`KismetMathLibrary.MakeTransform` (0.0 0.0 0.0)) "Undefined" "OverrideRootScale" null (`/Game/Core/Interactables/BPFL_RadialMenu.EnumToStaticMesh` (`.Type` (defaults `Object` (`|GetArrayItem` (`self.SubPawns_`) (`local.IconIndex`))))) (`KismetMathLibrary.MapRangeClamped` _returnvalue 0.0 360.0 0.0 1.0) null))
  (`KismetArrayLibrary.Array_Set` (`self.IconArray`) (`local.IconIndex`) _returnvalue_3 true)
  (`SceneComponent.K2_AttachToComponent` (`Actor.RootComponent` _returnvalue_3) _returnvalue_2 "None" "KeepRelative" "KeepRelative" "KeepRelative" false))

(fn `BuildRadialIcons`
  (params (SubClasses :type "Array of /Game/Core/Characters/BP_MasterPawn Class Reference"))
  (bind _returnvalue (`KismetArrayLibrary.Array_Length` SubClasses))
  (set `self.AngleBetweenIcons` (/ 360.0 (`KismetMathLibrary.Conv_IntToDouble` _returnvalue)))
  (for _index (range _returnvalue)
    (`self.AddNewIcon` _index (`self.SubPawns_`))))

(fn `UserConstructionScript`
  (bind _returnvalue (`PrimitiveComponent.CreateDynamicMaterialInstance` (`self.MenuGraphic`) 0 "/Game/MaterialLibrary/GUI/M_RadialLocations.M_RadialLocations" "None"))
  (set `self.MenuGraphicMaterial` _returnvalue))