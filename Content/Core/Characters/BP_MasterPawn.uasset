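; VR player pawn that picks a sub-pawn from a motion-controller radial menu and fires a matching projectile.
; BeginPlay attaches a hidden BP_RadialMenu built from SubPawns, toggled by the Magic Leap right home button.
; Either thumbstick's angle sets CurrentIcon and drives menu highlighting, with a center deadzone that deselects.
; The right trigger fires a reused, controller-attached BP_Projectile using the selection's mesh and an index-based hue shift.
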(event `Key|MagicLeap_Right_HomeButton`
  (params (Key :type "Key Structure"))
  (bind _radialmenu (`self.RadialMenu`))
  (:`Pressed`
    (`/Engine/EditorBlueprintResources/StandardMacros.IsValid` (`self.RadialMenu`)
      (:`Is Valid`
        (`/Engine/EditorBlueprintResources/StandardMacros.FlipFlop`
          (:`A`
            (`/Game/Core/Interactables/BP_RadialMenu.Reveal` _radialmenu))
          (:`B`
            (`/Game/Core/Interactables/BP_RadialMenu.Hide` _radialmenu)))))))

(event `self.ReceiveBeginPlay`
  (bind _returnvalue (`SceneComponent.K2_GetComponentToWorld` (`self.XRControl`)))
  (set `MotionControllerComponent.MotionSource` "AnyHand" (`self.XRControl`))
  (bind _returnvalue_2 (`|SpawnActorFromClass` "/Game/Core/Interactables/BP_RadialMenu.BP_RadialMenu_C" (`KismetMathLibrary.MakeTransform` (.location _returnvalue) (`KismetMathLibrary.MakeRotator` (.roll (.rotation _returnvalue)) (+ (.pitch (.rotation _returnvalue)) 15.0) (.yaw (.rotation _returnvalue)))) "Undefined" "OverrideRootScale" null null))
  (bind _output_get (set `self.RadialMenu` _returnvalue_2))
  (`/Game/Core/Interactables/BP_RadialMenu.Hide` _output_get)
  (`/Game/Core/Interactables/BP_RadialMenu.BuildRadialIcons` _output_get (`self.SubPawns`))
  (`self.K2_AttachToComponent` _output_get (`self.XRControl`) "None" "KeepRelative" "KeepRelative" "KeepRelative" true))

(event `Key|MotionController_Right_Shoulder`
  (params (Key :type "Key Structure")))

(event `Key|MagicLeap_Right_HomeButton`
  (params (Key :type "Key Structure")))

(event `InputAxisKey|MotionController_Right_Thumbstick_X`
  (params (AxisValue :type "Float (single-precision)"))
  (`self.UpdateRadialMenu` AxisValue (`self.GetInputAxisKeyValue`)))

(event `InputAxisKey|MotionController_Left_Thumbstick_X`
  (params (AxisValue :type "Float (single-precision)"))
  (`self.UpdateRadialMenu` AxisValue (`self.GetInputAxisKeyValue`)))

(event `Key|MotionController_Right_Trigger`
  (params (Key :type "Key Structure"))
  (:`Pressed`
    (`/Engine/EditorBlueprintResources/StandardMacros.IsValid` (`self.Projectile`)
      (:`Is Valid`
        _)
      (:`Is Not Valid`
        (bind _returnvalue (`|SpawnActorFromClass` "/Game/Core/BP_Projectile.BP_Projectile_C" (`SceneComponent.K2_GetComponentToWorld` (`self.XRControl`)) "Undefined" "OverrideRootScale" null null null))
        (bind _output_get (set `self.Projectile` _returnvalue))
        (`self.K2_AttachToComponent` _output_get (`self.XRControl`) "None" "SnapToTarget" "SnapToTarget" "SnapToTarget" false)))
    (`/Game/Core/BP_Projectile.FireProjectile` (`self.Projectile`) (`/Game/Core/Interactables/BPFL_RadialMenu.EnumToStaticMesh` (`.Type` (defaults `Object` (`|GetArrayItem` (`self.SubPawns`) (`self.CurrentIcon`))))) (* (`self.CurrentIcon`) (/ 1.0 (`KismetMathLibrary.Conv_IntToDouble` (`KismetArrayLibrary.Array_Length` (`self.SubPawns`))))))))

(fn `UpdateRadialMenu`
  (params (ThumbLocation_X :type "Float (double-precision)") (ThumbLocation_Y :type "Float (double-precision)"))
  (bind _returnvalue (`KismetMathLibrary.VSizeXY` (`KismetMathLibrary.MakeVector` ThumbLocation_X ThumbLocation_Y)))
  (bind _radialmenu (`self.RadialMenu`))
  (bind _radialmenu_2 (`self.RadialMenu`))
  (bind _currenticon (`self.CurrentIcon`))
  (bind _returnvalue_2 (`KismetArrayLibrary.Array_Length` (`self.SubPawns`)))
  (bind _returnvalue_3 (`KismetMathLibrary.DegAtan2` (`local.ThumbLocation_X`) (`local.ThumbLocation_Y`)))
  (bind _returnvalue_4 (mod (`KismetMathLibrary.Round` (/ (+ _returnvalue_3 (* (/ (- (`KismetMathLibrary.SignOfFloat` _returnvalue_3) 1.0) 2.0) -360.0)) (/ 360.0 (`KismetMathLibrary.Conv_IntToDouble` _returnvalue_2)))) _returnvalue_2))
  (if (!= _returnvalue 0.0)
    (if (< _returnvalue 0.4)
      (set `self.CurrentIcon` -1)
      (`/Engine/EditorBlueprintResources/StandardMacros.IsValid` _radialmenu
        (:`Is Valid`
          (`/Game/Core/Interactables/BP_RadialMenu.UpdateMaterial` _radialmenu (`KismetMathLibrary.MakeVector2D` (`local.ThumbLocation_X`) (`local.ThumbLocation_Y`)) true 0)
          (`/Game/Core/Interactables/BP_RadialMenu.Deselect` _radialmenu)))
      (else
        (if (!= _currenticon _returnvalue_4)
          (set `self.CurrentIcon` _returnvalue_4)
          (`/Engine/EditorBlueprintResources/StandardMacros.IsValid` _radialmenu_2
            (:`Is Valid`
              (`TextRenderComponent.K2_SetText` (`self.TextRender`) (`KismetTextLibrary.Conv_DoubleToText` (`KismetMathLibrary.Conv_IntToDouble` _currenticon) "HalfToEven"))
              (`/Game/Core/Interactables/BP_RadialMenu.ResizeIcons` (`self.RadialMenu`) (`self.CurrentIcon`))))
          (else
            (`/Engine/EditorBlueprintResources/StandardMacros.IsValid` _radialmenu_2
              (:`Is Valid`
                _))))
        (`/Game/Core/Interactables/BP_RadialMenu.UpdateMaterial` (`self.RadialMenu`) (`KismetMathLibrary.MakeVector2D` (`local.ThumbLocation_X`) (`local.ThumbLocation_Y`)) false (`self.CurrentIcon`))))))

(fn `UserConstructionScript`)