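; Master XR pawn that gives the player a motion-controller-driven radial menu.
; On BeginPlay it spawns a hidden BP_RadialMenu fed by DT_SUB_ACTORS and attaches it to the XRControl component.
; Right thumbstick, shoulder and trigger forward navigation, selection and actions to the menu, and the Magic Leap home button goes back.
; The pawn's own UpdateRadialMenu is an empty stub, with older angle-based selection, reveal toggle and possession logic left disconnected.
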(event `Key|MotionController_Right_Shoulder`
  (params (Key :type "Key Structure")))

(event `Key|MagicLeap_Right_HomeButton`
  (params (Key :type "Key Structure"))
  (:`Pressed`
    (`/RadialMenu/BP_RadialMenu.GoBack` (`self.RadialMenu`))))

(event `self.ReceiveBeginPlay`
  (bind _returnvalue (`SceneComponent.K2_GetComponentToWorld` (`self.XRControl`)))
  (bind _returnvalue_2 (`|SpawnActorFromClass` "/RadialMenu/BP_RadialMenu.BP_RadialMenu_C" (`KismetMathLibrary.MakeTransform` (.location _returnvalue) (`KismetMathLibrary.MakeRotator` (.roll (.rotation _returnvalue)) (+ (.pitch (.rotation _returnvalue)) 15.0) (.yaw (.rotation _returnvalue)))) "Undefined" "OverrideRootScale" null 0.25 "/RadialMenu/DT_SUB_ACTORS.DT_SUB_ACTORS" "Example" null))
  (bind _output_get (set `self.RadialMenu` _returnvalue_2))
  (`/RadialMenu/BP_RadialMenu.Hide` _output_get)
  (`self.K2_AttachToComponent` _output_get (`self.XRControl`) "None" "KeepRelative" "KeepRelative" "KeepRelative" true))

(event `Key|MagicLeap_Right_HomeButton`
  (params (Key :type "Key Structure")))

(event `InputAxisKey|MotionController_Right_Thumbstick_X`
  (params (AxisValue :type "Float (single-precision)")))

(event `InputAxisKey|MotionController_Right_Thumbstick_X`
  (params (AxisValue :type "Float (single-precision)"))
  (`/RadialMenu/BP_RadialMenu.UpdateRadialMenu` (`self.RadialMenu`) AxisValue (`self.GetInputAxisKeyValue`)))

(event `InputAxisKey|MotionController_Right_Thumbstick_Y`
  (params (AxisValue :type "Float (single-precision)")))

(event `Key|MotionController_Right_Shoulder`
  (params (Key :type "Key Structure"))
  (:`Pressed`
    (`/RadialMenu/BP_RadialMenu.ShoulderSelect` (`self.RadialMenu`))))

(event `Key|MotionController_Right_Trigger`
  (params (Key :type "Key Structure"))
  (:`Pressed`
    (`/RadialMenu/BP_RadialMenu.TriggerAction` (`self.RadialMenu`) (`SceneComponent.K2_GetComponentToWorld` (`self.XRControl`)))))

(fn `UpdateRadialMenu`
  (params (ThumbLocation_X :type "Float (double-precision)") (ThumbLocation_Y :type "Float (double-precision)")))

(fn `UserConstructionScript`)